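; RunController is a controller Blueprint for the RunCharacter pawn, with its logic left largely inactive.
; Tick reads the ShopInstance Stage1Complete flag and the pause state, but takes no action on either.
; An unconnected RotateToFaceCursor function would bank the character's roll left, right or level by the sign of its Y velocity, without reading the cursor despite its name.
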(event EventBeginPlay)

(event EventTick
  (params (DeltaSeconds :type Float%20%28single-precision%29))
  (bind _asshop_instance (Utilities|Casting|CastToShopInstance (Game|GetGameInstance)))
  (if (not (Variables|/Game/SFTS/Blueprints/ShopInstance.ShopInstance_C|GetStage1Complete _asshop_instance))
    (if (Variables|Default|GetGamePaused)
      _)))

(fn ConstructionScript)

(fn RotatetoFaceCursor
  (bind _returnvalue (Pawn|GetControlledPawn))
  (bind _returnvalue_2 (Transformation|GetVelocity _returnvalue))
  ;[1 1 1] Rotates the player to face a location based off the mouse in the distance and the direction the player is moving in
  (bind _asrun_character (Utilities|Casting|CastToRunCharacter _returnvalue))
  (if (< (.y _returnvalue_2) 0.0)
    (Variables|Default|SetRoll -4e+01)
    (elif (> (.y _returnvalue_2) 0.0)
      (Variables|Default|SetRoll 4e+01)
      (else
        (Variables|Default|SetRoll 0.0))))
  (Transformation|SetActorRotation _asrun_character (Math|Rotator|MakeRotator (Variables|Default|GetRoll) 0.0 0.0)))