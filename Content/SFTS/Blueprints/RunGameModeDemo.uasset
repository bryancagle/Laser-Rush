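; RunGameModeDemo is a game mode Blueprint, apparently for a runner demo, that lays a track of blank demo floor tiles at BeginPlay.
; AddStarterFloorTile spawns BP_FloorBlankDemo at NextSpawnPoint, then stores that tile's attach transform as the next spawn point, chaining tiles end to end.
; AddFloorTile does the same with BP_FloorTile, but nothing in this Blueprint calls it.
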(event EventBeginPlay
  (CallFunction|AddStarterFloorTile)
  (for _index (range 0 9)
    (CallFunction|AddStarterFloorTile)))

(fn ConstructionScript)

(fn AddFloorTile
  (bind _returnvalue (Game|SpawnActorfromClass "/Game/SFTS/Blueprints/EarthZone/BP_FloorTile.BP_FloorTile_C" (Variables|Default|GetNextSpawnPoint) "Undefined" 0 0))
  (bind _attachtransform (Default|GetAttachTransform _returnvalue))
  (Variables|Default|SetNextSpawnPoint _attachtransform))

(fn AddStarterFloorTile
  (bind _returnvalue (Game|SpawnActorfromClass "/Game/SFTS/Blueprints/EarthZone/BP_FloorBlankDemo.BP_FloorBlankDemo_C" (Variables|Default|GetNextSpawnPoint) "Undefined" 0 0))
  (bind _attachtransform (Default|GetAttachTransform _returnvalue))
  (Variables|Default|SetNextSpawnPoint _attachtransform))