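; Blank floor tile for the endless runner demo, chained to the next tile through the transform of its AttachPoint.
; Construction adds a child actor at each of two border spawn points; SetSpawnPoints is an empty stub.
; When RunCharacterDemo overlaps EndTrigger, the tile asks RunGameModeDemo to add a starter floor tile, then destroys itself after a short delay.
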(event OnComponentBeginOverlap(EndTrigger)
  (params (OverlappedComponent :type Primitive%20Component%20Object%20Reference) (OtherActor :type Actor%20Object%20Reference) (OtherComp :type Primitive%20Component%20Object%20Reference) (OtherBodyIndex :type Integer) (bFromSweep :type Boolean) (SweepResult :type Hit%20Result%20Structure%20%28by%20ref%29))
  ;[1 1 1] When the player crosses the trigger, a floor will be spawned and delete an older one
  (Utilities|Casting|CastToRunCharacterDemo OtherActor)
  (bind _asrun_game_mode_demo (Utilities|Casting|CastToRunGameModeDemo (Game|GetGameMode)))
  (Default|AddStarterFloorTile _asrun_game_mode_demo)
  (Utilities|FlowControl|Delay 1.0)
  (Actor|DestroyActor))

(event EventBeginPlay)

(event Collision|EventActorBeginOverlap
  (params (OtherActor :type Actor%20Object%20Reference)))

(event EventTick
  (params (DeltaSeconds :type Float%20%28single-precision%29)))

(fn ConstructionScript
  (CallFunction|SetSpawnPoints)
  (CallFunction|SpawnBlocker))

(fn GetAttachTransform
  ;[1 1 1] Attaches one segment of ground to the next
  (return (Transformation|GetWorldTransform (Variables|Default|GetAttachPoint))))

(fn SetSpawnPoints)

(fn SpawnBlocker
  ;[1 1 1] A random rock obstacle is placed
  (AddComponent|AddChildActorComponent false (Transformation|GetRelativeTransform (Variables|Default|GetBorderSpawnPoint)))
  (AddComponent|AddChildActorComponent false (Transformation|GetRelativeTransform (Variables|Default|GetBorderSpawnPoint2))))