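; Blocker3 is a destructible rock obstacle in the runner's EarthZone.
; Hitting its mesh damages the RunCharacter and passes the hit normal's Y as knockback direction.
; RockDamaged subtracts the player's damage output from health set in the construction script, while BoostedThrough destroys it outright.
; Both destruction paths hide the mesh, spawn a scaled explosion, and add random stardust and fixed score to ShopInstance before destroying the actor.
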(event OnComponentHit(StaticMesh)
  (params (HitComponent :type Primitive%20Component%20Object%20Reference) (OtherActor :type Actor%20Object%20Reference) (OtherComp :type Primitive%20Component%20Object%20Reference) (NormalImpulse :type Vector :default "0, 0, 0") (Hit :type Hit%20Result%20Structure%20%28by%20ref%29))
  ;[1 1 1] The player dies when a direct impact is made, to be set to do damage instead of one hit kill. Also sets what direction the player will fly in
  (bind _asrun_character (Utilities|Casting|CastToRunCharacter OtherActor))
  (Variables|/Game/SFTS/Blueprints/RunCharacter.RunCharacter_C|SetHitDirection _asrun_character (.y (.normal Hit)))
  (Default|PlayerDamage _asrun_character))

(event Custom|RockDamaged
  (bind _returnvalue (Transformation|GetActorLocation))
  ;[1 1 1] When destroy event is called, the visibility and collision are turned off, and an explosion is placed
  (Variables|Default|SetHealth (- (Variables|Default|GetHealth) (Variables|/Game/SFTS/Blueprints/RunCharacter.RunCharacter_C|GetDamageOutput (Variables|Default|GetPlayer))))
  (if (<= (Variables|Default|GetHealth) 0.0)
    (Rendering|SetVisibility (Variables|Default|GetStaticMesh) false false)
    (Collision|SetCollisionEnabled (Variables|Default|GetStaticMesh) "NoCollision")
    (bind _returnvalue_2 (Effects|SpawnEmitteratLocation "/Game/StarterContent/Particles/P_Explosion.P_Explosion" (Math|Vector|MakeVector (.x _returnvalue) (.y _returnvalue) (+ (.z _returnvalue) 1.7e+02)) "0.000000, 0, 0"))
    (Transformation|SetRelativeScale3D _returnvalue_2 "4.000000,4.000000,4.000000")
    (bind _asshop_instance (Utilities|Casting|CastToShopInstance (Game|GetGameInstance)))
    (Variables|/Game/SFTS/Blueprints/ShopInstance.ShopInstance_C|SetCurrentStardust _asshop_instance (+ (Variables|/Game/SFTS/Blueprints/ShopInstance.ShopInstance_C|GetCurrentStardust _asshop_instance) (Math|Random|RandomIntegerinRange 50 150)))
    (Variables|/Game/SFTS/Blueprints/ShopInstance.ShopInstance_C|SetCurrentScore _asshop_instance (+ (Variables|/Game/SFTS/Blueprints/ShopInstance.ShopInstance_C|GetCurrentScore _asshop_instance) 100))
    (Actor|DestroyActor)))

(event Custom|BoostedThrough
  (bind _returnvalue (Transformation|GetActorLocation))
  ;[1 1 1] When destroy event is called, the visibility and collision are turned off, and an explosion is placed
  (Rendering|SetVisibility (Variables|Default|GetStaticMesh) false false)
  (Collision|SetCollisionEnabled (Variables|Default|GetStaticMesh) "NoCollision")
  (bind _returnvalue_2 (Effects|SpawnEmitteratLocation "/Game/StarterContent/Particles/P_Explosion.P_Explosion" (Math|Vector|MakeVector (.x _returnvalue) (.y _returnvalue) (+ (.z _returnvalue) 1.7e+02)) "0.000000, 0, 0"))
  (Transformation|SetRelativeScale3D _returnvalue_2 "4.000000,4.000000,4.000000")
  (bind _asshop_instance (Utilities|Casting|CastToShopInstance (Game|GetGameInstance)))
  (Variables|/Game/SFTS/Blueprints/ShopInstance.ShopInstance_C|SetCurrentStardust _asshop_instance (+ (Variables|/Game/SFTS/Blueprints/ShopInstance.ShopInstance_C|GetCurrentStardust _asshop_instance) (Math|Random|RandomIntegerinRange 50 150)))
  (Variables|/Game/SFTS/Blueprints/ShopInstance.ShopInstance_C|SetCurrentScore _asshop_instance (+ (Variables|/Game/SFTS/Blueprints/ShopInstance.ShopInstance_C|GetCurrentScore _asshop_instance) 100))
  (Actor|DestroyActor))

(event EventBeginPlay
  (bind _asrun_character (Utilities|Casting|CastToRunCharacter (Game|GetPlayerCharacter 0)))
  (Variables|Default|SetPlayer _asrun_character))

(event Collision|EventActorBeginOverlap
  (params (OtherActor :type Actor%20Object%20Reference)))

(event EventTick
  (params (DeltaSeconds :type Float%20%28single-precision%29)))

(fn ConstructionScript
  (Variables|Default|SetHealth 8.0))