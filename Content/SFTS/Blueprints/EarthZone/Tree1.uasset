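; Tree obstacle Blueprint for the Earth zone that damages the RunCharacter on contact and rewards being boosted through.
; A component hit on the tree mesh stores the impact's Y location as the character's HitDirection, then calls PlayerDamage.
; The BoostedThrough event hides the tree, disables its collision, spawns a scaled-up explosion and adds random stardust plus fixed score to ShopInstance, the game instance.
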(event OnComponentHit(Tree1)
  (params (HitComponent :type Primitive%20Component%20Object%20Reference) (OtherActor :type Actor%20Object%20Reference) (OtherComp :type Primitive%20Component%20Object%20Reference) (NormalImpulse :type Vector :default "0, 0, 0") (Hit :type Hit%20Result%20Structure%20%28by%20ref%29))
  (bind _asrun_character (Utilities|Casting|CastToRunCharacter OtherActor))
  (Variables|/Game/SFTS/Blueprints/RunCharacter.RunCharacter_C|SetHitDirection _asrun_character (.y (.location Hit)))
  (Default|PlayerDamage _asrun_character))

(event Custom|BoostedThrough
  (bind _returnvalue (Transformation|GetActorLocation))
  (bind _tree1 (Variables|Default|GetTree1))
  (Rendering|SetVisibility _tree1 false false)
  (Collision|SetCollisionEnabled _tree1 "NoCollision")
  (bind _returnvalue_2 (Effects|SpawnEmitteratLocation "/Game/StarterContent/Particles/P_Explosion.P_Explosion" (Math|Vector|MakeVector (.x _returnvalue) (.y _returnvalue) (+ (.z _returnvalue) 1.7e+02)) "0.000000, 0, 0"))
  (Transformation|SetRelativeScale3D _returnvalue_2 "4.000000,4.000000,4.000000")
  (bind _asshop_instance (Utilities|Casting|CastToShopInstance (Game|GetGameInstance)))
  (Variables|/Game/SFTS/Blueprints/ShopInstance.ShopInstance_C|SetCurrentStardust _asshop_instance (+ (Variables|/Game/SFTS/Blueprints/ShopInstance.ShopInstance_C|GetCurrentStardust _asshop_instance) (Math|Random|RandomIntegerinRange 50 150)))
  (Variables|/Game/SFTS/Blueprints/ShopInstance.ShopInstance_C|SetCurrentScore _asshop_instance (+ (Variables|/Game/SFTS/Blueprints/ShopInstance.ShopInstance_C|GetCurrentScore _asshop_instance) 100)))

(event EventBeginPlay
  (bind _asrun_character (Utilities|Casting|CastToRunCharacter (Game|GetPlayerCharacter 0)))
  (Variables|Default|SetPlayer _asrun_character))

(event Collision|EventActorBeginOverlap
  (params (OtherActor :type Actor%20Object%20Reference)))

(event EventTick
  (params (DeltaSeconds :type Float%20%28single-precision%29)))

(fn ConstructionScript)