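; Collectible diamond pickup that registers itself with ShopInstance on spawn and spins until the RunCharacter overlaps its sphere.
; Pickup adds score and diamond count, plays a sound, then shrinks the mesh and lifts it above the player before the actor self-destroys.
; With DDAMode on, each pickup also raises GameDifficulty by a tier-based step that shrinks at higher tiers, tracks PeakDifficulty, and boosts the player's clamped FlySpeed.
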(event OnComponentBeginOverlap(Sphere)
  (params (OverlappedComponent :type Primitive%20Component%20Object%20Reference) (OtherActor :type Actor%20Object%20Reference) (OtherComp :type Primitive%20Component%20Object%20Reference) (OtherBodyIndex :type Integer) (bFromSweep :type Boolean) (SweepResult :type Hit%20Result%20Structure%20%28by%20ref%29))
  (Utilities|Casting|CastToRunCharacter OtherActor)
  (bind _asshop_instance (Utilities|Casting|CastToShopInstance (Game|GetGameInstance)))
  (Variables|/Game/SFTS/Blueprints/ShopInstance.ShopInstance_C|SetCurrentScore _asshop_instance (+ (Variables|/Game/SFTS/Blueprints/ShopInstance.ShopInstance_C|GetCurrentScore _asshop_instance) 100))
  (Variables|/Game/SFTS/Blueprints/ShopInstance.ShopInstance_C|SetDiamondCount _asshop_instance (+ (Variables|/Game/SFTS/Blueprints/ShopInstance.ShopInstance_C|GetDiamondCount _asshop_instance) 1))
  (bind _output_get (Variables|Default|SetCurrentDifficulty (Math|Float|Floor (Variables|/Game/SFTS/Blueprints/ShopInstance.ShopInstance_C|GetGameDifficulty _asshop_instance))))
  (if (Variables|/Game/SFTS/Blueprints/ShopInstance.ShopInstance_C|GetDDA%20Mode _asshop_instance)
    (switch int _output_get
      (:1
        (Variables|/Game/SFTS/Blueprints/ShopInstance.ShopInstance_C|SetGameDifficulty _asshop_instance (Math|Float|Clamp(Float) (+ (Variables|/Game/SFTS/Blueprints/ShopInstance.ShopInstance_C|GetGameDifficulty _asshop_instance) 0.22) 1.0 1e+01)))
      (:2
        (Variables|/Game/SFTS/Blueprints/ShopInstance.ShopInstance_C|SetGameDifficulty _asshop_instance (Math|Float|Clamp(Float) (+ (Variables|/Game/SFTS/Blueprints/ShopInstance.ShopInstance_C|GetGameDifficulty _asshop_instance) 0.21) 1.0 1e+01)))
      (:3
        (Variables|/Game/SFTS/Blueprints/ShopInstance.ShopInstance_C|SetGameDifficulty _asshop_instance (Math|Float|Clamp(Float) (+ (Variables|/Game/SFTS/Blueprints/ShopInstance.ShopInstance_C|GetGameDifficulty _asshop_instance) 0.2) 1.0 1e+01)))
      (:4
        (Variables|/Game/SFTS/Blueprints/ShopInstance.ShopInstance_C|SetGameDifficulty _asshop_instance (Math|Float|Clamp(Float) (+ (Variables|/Game/SFTS/Blueprints/ShopInstance.ShopInstance_C|GetGameDifficulty _asshop_instance) 0.18) 1.0 1e+01)))
      (:5
        (Variables|/Game/SFTS/Blueprints/ShopInstance.ShopInstance_C|SetGameDifficulty _asshop_instance (Math|Float|Clamp(Float) (+ (Variables|/Game/SFTS/Blueprints/ShopInstance.ShopInstance_C|GetGameDifficulty _asshop_instance) 0.16) 1.0 1e+01)))
      (:6
        (Variables|/Game/SFTS/Blueprints/ShopInstance.ShopInstance_C|SetGameDifficulty _asshop_instance (Math|Float|Clamp(Float) (+ (Variables|/Game/SFTS/Blueprints/ShopInstance.ShopInstance_C|GetGameDifficulty _asshop_instance) 0.13) 1.0 1e+01)))
      (:7
        (Variables|/Game/SFTS/Blueprints/ShopInstance.ShopInstance_C|SetGameDifficulty _asshop_instance (Math|Float|Clamp(Float) (+ (Variables|/Game/SFTS/Blueprints/ShopInstance.ShopInstance_C|GetGameDifficulty _asshop_instance) 0.11) 1.0 1e+01)))
      (:8
        (Variables|/Game/SFTS/Blueprints/ShopInstance.ShopInstance_C|SetGameDifficulty _asshop_instance (Math|Float|Clamp(Float) (+ (Variables|/Game/SFTS/Blueprints/ShopInstance.ShopInstance_C|GetGameDifficulty _asshop_instance) 0.09) 1.0 1e+01)))
      (:9
        (Variables|/Game/SFTS/Blueprints/ShopInstance.ShopInstance_C|SetGameDifficulty _asshop_instance (Math|Float|Clamp(Float) (+ (Variables|/Game/SFTS/Blueprints/ShopInstance.ShopInstance_C|GetGameDifficulty _asshop_instance) 0.07) 1.0 1e+01)))
      (:10
        (Variables|/Game/SFTS/Blueprints/ShopInstance.ShopInstance_C|SetGameDifficulty _asshop_instance (Math|Float|Clamp(Float) (+ (Variables|/Game/SFTS/Blueprints/ShopInstance.ShopInstance_C|GetGameDifficulty _asshop_instance) 0.05) 1.0 1e+01))))
    (if (>= (Variables|/Game/SFTS/Blueprints/ShopInstance.ShopInstance_C|GetGameDifficulty _asshop_instance) (Variables|/Game/SFTS/Blueprints/ShopInstance.ShopInstance_C|GetPeakDifficulty _asshop_instance))
      (Variables|/Game/SFTS/Blueprints/ShopInstance.ShopInstance_C|SetPeakDifficulty _asshop_instance (Variables|/Game/SFTS/Blueprints/ShopInstance.ShopInstance_C|GetGameDifficulty _asshop_instance))))
  (Variables|Default|SetIsCollected true)
  (bind _asrun_character (Utilities|Casting|CastToRunCharacter (Game|GetPlayerCharacter 0)))
  (Transformation|SetWorldLocation (Variables|Default|GetStaticMesh1) (Math|Vector|MakeVector (.x (Transformation|GetWorldLocation (Variables|/Script/Engine.Character|GetCapsuleComponent _asrun_character))) (.y (Transformation|GetWorldLocation (Variables|/Script/Engine.Character|GetCapsuleComponent _asrun_character))) (- (.z (Transformation|GetWorldLocation (Variables|/Script/Engine.Character|GetCapsuleComponent _asrun_character))) 3e+01)) false false)
  (Audio|PlaySound2D "/Game/SFTS/Audio/DiamondSound.DiamondSound")
  (bind _asshop_instance_2 (Utilities|Casting|CastToShopInstance (Game|GetGameInstance)))
  (bind _output_get_2 (Variables|Default|SetCurrentDifficulty (Math|Float|Floor (Variables|/Game/SFTS/Blueprints/ShopInstance.ShopInstance_C|GetGameDifficulty _asshop_instance_2))))
  (if (Variables|/Game/SFTS/Blueprints/ShopInstance.ShopInstance_C|GetDDA%20Mode _asshop_instance_2)
    (switch int _output_get_2
      (:1
        (bind _output_get_3 (Variables|/Game/SFTS/Blueprints/RunCharacter.RunCharacter_C|SetFlySpeed _asrun_character (+ 3e+01 (Variables|/Game/SFTS/Blueprints/RunCharacter.RunCharacter_C|GetFlySpeed _asrun_character)))))
      (:2
        (Variables|/Game/SFTS/Blueprints/RunCharacter.RunCharacter_C|SetFlySpeed _asrun_character (+ 4e+01 (Variables|/Game/SFTS/Blueprints/RunCharacter.RunCharacter_C|GetFlySpeed _asrun_character))))
      (:3
        (Variables|/Game/SFTS/Blueprints/RunCharacter.RunCharacter_C|SetFlySpeed _asrun_character (+ 4e+01 (Variables|/Game/SFTS/Blueprints/RunCharacter.RunCharacter_C|GetFlySpeed _asrun_character))))
      (:4
        (Variables|/Game/SFTS/Blueprints/RunCharacter.RunCharacter_C|SetFlySpeed _asrun_character (+ 45.0 (Variables|/Game/SFTS/Blueprints/RunCharacter.RunCharacter_C|GetFlySpeed _asrun_character))))
      (:5
        (Variables|/Game/SFTS/Blueprints/RunCharacter.RunCharacter_C|SetFlySpeed _asrun_character (+ 5e+01 (Variables|/Game/SFTS/Blueprints/RunCharacter.RunCharacter_C|GetFlySpeed _asrun_character))))
      (:6
        (Variables|/Game/SFTS/Blueprints/RunCharacter.RunCharacter_C|SetFlySpeed _asrun_character (+ 55.0 (Variables|/Game/SFTS/Blueprints/RunCharacter.RunCharacter_C|GetFlySpeed _asrun_character))))
      (:7
        (Variables|/Game/SFTS/Blueprints/RunCharacter.RunCharacter_C|SetFlySpeed _asrun_character (+ 6e+01 (Variables|/Game/SFTS/Blueprints/RunCharacter.RunCharacter_C|GetFlySpeed _asrun_character))))
      (:8
        (Variables|/Game/SFTS/Blueprints/RunCharacter.RunCharacter_C|SetFlySpeed _asrun_character (+ 65.0 (Variables|/Game/SFTS/Blueprints/RunCharacter.RunCharacter_C|GetFlySpeed _asrun_character))))
      (:9
        (Variables|/Game/SFTS/Blueprints/RunCharacter.RunCharacter_C|SetFlySpeed _asrun_character (+ 7e+01 (Variables|/Game/SFTS/Blueprints/RunCharacter.RunCharacter_C|GetFlySpeed _asrun_character))))
      (:10
        (Variables|/Game/SFTS/Blueprints/RunCharacter.RunCharacter_C|SetFlySpeed _asrun_character (+ 75.0 (Variables|/Game/SFTS/Blueprints/RunCharacter.RunCharacter_C|GetFlySpeed _asrun_character)))))
    (Variables|/Game/SFTS/Blueprints/RunCharacter.RunCharacter_C|SetFlySpeed _asrun_character (Math|Float|Clamp(Float) _output_get_3 3e+03 6.5e+03))))

(event EventBeginPlay
  (bind _asshop_instance (Utilities|Casting|CastToShopInstance (Game|GetGameInstance)))
  (Variables|/Game/SFTS/Blueprints/ShopInstance.ShopInstance_C|SetDiamondsSpawned _asshop_instance (+ (Variables|/Game/SFTS/Blueprints/ShopInstance.ShopInstance_C|GetDiamondsSpawned _asshop_instance) 1)))

(event Collision|EventActorBeginOverlap
  (params (OtherActor :type Actor%20Object%20Reference)))

(event EventTick
  (params (DeltaSeconds :type Float%20%28single-precision%29))
  (bind _staticmesh1 (Variables|Default|GetStaticMesh1))
  (bind _staticmesh1_2 (Variables|Default|GetStaticMesh1))
  (bind _relativerotation (Variables|/Script/Engine.SceneComponent|GetRelativeRotation _staticmesh1))
  (bind _relativerotation_2 (Variables|/Script/Engine.SceneComponent|GetRelativeRotation _staticmesh1_2))
  (if (Variables|Default|GetIsCollected)
    (bind _asrun_character (Utilities|Casting|CastToRunCharacter (Game|GetPlayerCharacter 0)))
    (Transformation|SetWorldLocation (Variables|Default|GetStaticMesh1) (Math|Vector|MakeVector (.x (Transformation|GetWorldLocation (Variables|/Script/Engine.Character|GetCapsuleComponent _asrun_character))) (.y (Transformation|GetWorldLocation (Variables|/Script/Engine.Character|GetCapsuleComponent _asrun_character))) (.z (Math|Interpolation|VInterpTo (Transformation|GetWorldLocation (Variables|Default|GetStaticMesh1)) (Math|Vector|MakeVector 0.0 0.0 (+ (.z (Transformation|GetWorldLocation (Variables|/Script/Engine.Character|GetCapsuleComponent _asrun_character))) 1.5e+02)) 0.1 2.0))) false false)
    (Transformation|SetRelativeScale3D (Variables|Default|GetStaticMesh1) "0.300000,0.300000,0.300000")
    (Transformation|SetRelativeRotation _staticmesh1 (Math|Rotator|MakeRotator (.roll _relativerotation) (.pitch _relativerotation) (+ (.yaw _relativerotation) 8.0)) false false)
    (Utilities|FlowControl|Delay 0.5)
    (bind _output_get (Variables|Default|Setdestroy%20timer (+ (Variables|Default|Getdestroy%20timer) 1)))
    (if (== _output_get 1)
      (Actor|DestroyActor))
    (else
      (Transformation|SetRelativeRotation _staticmesh1_2 (Math|Rotator|MakeRotator (.roll _relativerotation_2) (.pitch _relativerotation_2) (+ (.yaw _relativerotation_2) 8.0)) false false))))

(fn ConstructionScript)