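; Game mode for the EarthZone run that builds the starting floor track when play begins.
; On BeginPlay it spawns two blank starter tiles, then two regular floor tiles.
; Each spawn uses a stored next spawn point, which is then updated from the new tile's attach transform so the tiles chain end to end.
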(event EventBeginPlay
  (CallFunction|AddStarterFloorTile)
  (CallFunction|AddStarterFloorTile)
  (for _index (range 0 1)
    (CallFunction|AddFloorTile)))

(fn ConstructionScript)

(fn AddFloorTile
  (bind _returnvalue (Game|SpawnActorfromClass "/Game/SFTS/Blueprints/EarthZone/BP_FloorTile.BP_FloorTile_C" (Variables|Default|GetNextSpawnPoint) "Undefined" 0 0))
  (bind _attachtransform (Default|GetAttachTransform _returnvalue))
  (Variables|Default|SetNextSpawnPoint _attachtransform))

(fn AddStarterFloorTile
  (bind _returnvalue (Game|SpawnActorfromClass "/Game/SFTS/Blueprints/EarthZone/BP_FloorBlank.BP_FloorBlank_C" (Variables|Default|GetNextSpawnPoint) "Undefined" 0 0))
  (bind _attachtransform (Default|GetAttachTransform _returnvalue))
  (Variables|Default|SetNextSpawnPoint _attachtransform))