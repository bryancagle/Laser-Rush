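; Earth zone floor tile for an endless runner that populates itself with obstacles, borders and a diamond.
; Construction gathers spawn-point transforms, then adds child actors at random points, with obstacle and tree odds set by the game instance's difficulty.
; Crossing the end trigger asks the game mode for another tile, or a starter tile once the tile count passes a limit.
; The tile destroys itself after a delay unless the runner is in transition mode.
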(event OnComponentBeginOverlap(EndTrigger)
  (params (OverlappedComponent :type Primitive%20Component%20Object%20Reference) (OtherActor :type Actor%20Object%20Reference) (OtherComp :type Primitive%20Component%20Object%20Reference) (OtherBodyIndex :type Integer) (bFromSweep :type Boolean) (SweepResult :type Hit%20Result%20Structure%20%28by%20ref%29))
  ;[1 1 1] When the player crosses the trigger, a floor will be spawned and delete an older one
  (bind _asrun_character (Utilities|Casting|CastToRunCharacter OtherActor))
  (bind _asrun_game_mode (Utilities|Casting|CastToRunGameMode (Game|GetGameMode)))
  (bind _asshop_instance (Utilities|Casting|CastToShopInstance (Game|GetGameInstance)))
  (if (<= (Variables|/Game/SFTS/Blueprints/ShopInstance.ShopInstance_C|GetTilesSpawn _asshop_instance) 65)
    (Default|AddFloorTile _asrun_game_mode)
    (else
      (Default|AddStarterFloorTile _asrun_game_mode)))
  (Utilities|FlowControl|Delay 1.5)
  (if (not (Variables|/Game/SFTS/Blueprints/RunCharacter.RunCharacter_C|GetTransitionMode _asrun_character))
    (Actor|DestroyActor)))

(event EventBeginPlay)

(event Collision|EventActorBeginOverlap
  (params (OtherActor :type Actor%20Object%20Reference)))

(event EventTick
  (params (DeltaSeconds :type Float%20%28single-precision%29)))

(fn ConstructionScript
  (CallFunction|SetSpawnPoints)
  (CallFunction|SpawnBlocker))

(fn GetAttachTransform
  ;[1 1 1] Attaches one segment of ground to the next
  (return (Transformation|GetWorldTransform (Variables|Default|GetAttachPoint))))

(fn SetSpawnPoints
  ;[1 1 1] Creates an array of spawn points
  (Variables|Default|SetSpawnPoints (Utilities|Array|MakeArray (Transformation|GetRelativeTransform (Variables|Default|GetSpawnPoint1)) (Transformation|GetRelativeTransform (Variables|Default|GetSpawnPoint2)) (Transformation|GetRelativeTransform (Variables|Default|GetSpawnPoint3)) (Transformation|GetRelativeTransform (Variables|Default|GetSpawnPoint4)) (Transformation|GetRelativeTransform (Variables|Default|GetSpawnPoint5)) (Transformation|GetRelativeTransform (Variables|Default|GetSpawnPoint6)) (Transformation|GetRelativeTransform (Variables|Default|GetSpawnPoint7)) (Transformation|GetRelativeTransform (Variables|Default|GetSpawnPoint8)) (Transformation|GetRelativeTransform (Variables|Default|GetSpawnPoint9))))
  (Variables|Default|SetHorizontalSpawnPoints (Utilities|Array|MakeArray (Transformation|GetRelativeTransform (Variables|Default|GetHorizontalSpawnPoint1)) (Transformation|GetRelativeTransform (Variables|Default|GetHorizontalSpawnPoint2)) (Transformation|GetRelativeTransform (Variables|Default|GetHorizontalSpawnPoint3)) (Transformation|GetRelativeTransform (Variables|Default|GetHorizontalSpawnPoint4)) (Transformation|GetRelativeTransform (Variables|Default|GetHorizontalSpawnPoint5))))
  (Variables|Default|SetTreeSpawnPoints (Utilities|Array|MakeArray (Transformation|GetRelativeTransform (Variables|Default|GetTreeSpawnPoint5)) (Transformation|GetRelativeTransform (Variables|Default|GetTreeSpawnPoint2)) (Transformation|GetRelativeTransform (Variables|Default|GetTreeSpawnPoint3)) (Transformation|GetRelativeTransform (Variables|Default|GetTreeSpawnPoint4)) (Transformation|GetRelativeTransform (Variables|Default|GetTreeSpawnPoint1)) (Transformation|GetRelativeTransform (Variables|Default|GetTreeSpawnPoint6)) (Transformation|GetRelativeTransform (Variables|Default|GetTreeSpawnPoint7)) (Transformation|GetRelativeTransform (Variables|Default|GetTreeSpawnPoint8)) (Transformation|GetRelativeTransform (Variables|Default|GetTreeSpawnPoint9))))
  (Variables|Default|SetDiamondSpawnPoints (Utilities|Array|MakeArray (Transformation|GetRelativeTransform (Variables|Default|GetDiamondSpawnPoint14)) (Transformation|GetRelativeTransform (Variables|Default|GetDiamondSpawnPoint2)) (Transformation|GetRelativeTransform (Variables|Default|GetDiamondSpawnPoint3)) (Transformation|GetRelativeTransform (Variables|Default|GetDiamondSpawnPoint4)) (Transformation|GetRelativeTransform (Variables|Default|GetDiamondSpawnPoint5)) (Transformation|GetRelativeTransform (Variables|Default|GetDiamondSpawnPoint6)) (Transformation|GetRelativeTransform (Variables|Default|GetDiamondSpawnPoint7)) (Transformation|GetRelativeTransform (Variables|Default|GetDiamondSpawnPoint8)) (Transformation|GetRelativeTransform (Variables|Default|GetDiamondSpawnPoint9)) (Transformation|GetRelativeTransform (Variables|Default|GetDiamondSpawnPoint10)) (Transformation|GetRelativeTransform (Variables|Default|GetDiamondSpawnPoint11)) (Transformation|GetRelativeTransform (Variables|Default|GetDiamondSpawnPoint12)) (Transformation|GetRelativeTransform (Variables|Default|GetDiamondSpawnPoint13)) (Transformation|GetRelativeTransform (Variables|Default|GetDiamondSpawnPoint)) (Transformation|GetRelativeTransform (Variables|Default|GetDiamondSpawnPoint15)) (Transformation|GetRelativeTransform (Variables|Default|GetDiamondSpawnPoint16)) (Transformation|GetRelativeTransform (Variables|Default|GetDiamondSpawnPoint17)) (Transformation|GetRelativeTransform (Variables|Default|GetDiamondSpawnPoint18)) (Transformation|GetRelativeTransform (Variables|Default|GetDiamondSpawnPoint19)) (Transformation|GetRelativeTransform (Variables|Default|GetDiamondSpawnPoint20)) (Transformation|GetRelativeTransform (Variables|Default|GetDiamondSpawnPoint21)) (Transformation|GetRelativeTransform (Variables|Default|GetDiamondSpawnPoint22)) (Transformation|GetRelativeTransform (Variables|Default|GetDiamondSpawnPoint23)) (Transformation|GetRelativeTransform (Variables|Default|GetDiamondSpawnPoint24)) (Transformation|GetRelativeTransform (Variables|Default|GetDiamondSpawnPoint25)) (Transformation|GetRelativeTransform (Variables|Default|GetDiamondSpawnPoint26)) (Transformation|GetRelativeTransform (Variables|Default|GetDiamondSpawnPoint27)))))

(fn SpawnBlocker
  (bind _horizontalspawnpoints (Variables|Default|GetHorizontalSpawnPoints))
  (bind _treespawnpoints (Variables|Default|GetTreeSpawnPoints))
  (bind _treespawnpoints_2 (Variables|Default|GetTreeSpawnPoints))
  (bind _spawnpoints (Variables|Default|GetSpawnPoints))
  (bind _diamondspawnpoints (Variables|Default|GetDiamondSpawnPoints))
  ;[1 1 1] A random rock obstacle is placed
  (bind _asshop_instance (Utilities|Casting|CastToShopInstance (Game|GetGameInstance)))
  (bind _output_get (Variables|Default|SetCurrentDifficulty (Math|Float|Floor (Variables|/Game/SFTS/Blueprints/ShopInstance.ShopInstance_C|GetGameDifficulty _asshop_instance))))
  (switch int _output_get
    (:1
      (Variables|Default|SetSpawnPercent 0.25))
    (:2
      (Variables|Default|SetSpawnPercent 0.25))
    (:3
      (Variables|Default|SetSpawnPercent 0.3))
    (:4
      (Variables|Default|SetSpawnPercent 0.4))
    (:5
      (Variables|Default|SetSpawnPercent 0.5))
    (:6
      (Variables|Default|SetSpawnPercent 0.6))
    (:7
      (Variables|Default|SetSpawnPercent 0.7))
    (:8
      (Variables|Default|SetSpawnPercent 0.8))
    (:9
      (Variables|Default|SetSpawnPercent 0.9))
    (:10
      (Variables|Default|SetSpawnPercent 1.0)))
  (Utilities|FlowControl|Sequence
    (:then_0
      (if (Math|Random|RandomBoolwithWeight (Variables|Default|GetSpawnPercent))
        (AddComponent|AddChildActorComponent false (Utilities|Array|Get(acopy) _spawnpoints (Math|Random|RandomIntegerinRange 0 (Utilities|Array|LastIndex _spawnpoints))))))
    (:then_1
      (if (Math|Random|RandomBoolwithWeight (Variables|Default|GetSpawnPercent))
        (AddComponent|AddChildActorComponent false (Utilities|Array|Get(acopy) _horizontalspawnpoints (Math|Random|RandomIntegerinRange 0 (Utilities|Array|LastIndex _horizontalspawnpoints))))))
    (:then_2
      (if (Math|Random|RandomBoolwithWeight (Variables|Default|GetSpawnPercent))
        (AddComponent|AddChildActorComponent false (Utilities|Array|Get(acopy) _treespawnpoints_2 (Math|Random|RandomIntegerinRange 0 (Utilities|Array|LastIndex _treespawnpoints_2))))))
    (:then_3
      (if (Math|Random|RandomBoolwithWeight (Variables|Default|GetSpawnPercent))
        (AddComponent|AddChildActorComponent false (Utilities|Array|Get(acopy) _treespawnpoints (Math|Random|RandomIntegerinRange 0 (Utilities|Array|LastIndex _treespawnpoints))))))
    (:then_4
      (AddComponent|AddChildActorComponent false (Transformation|GetRelativeTransform (Variables|Default|GetBorderSpawnPoint)))
      (AddComponent|AddChildActorComponent false (Transformation|GetRelativeTransform (Variables|Default|GetBorderSpawnPoint2))))
    (:then_5
      (bind _asshop_instance_2 (Utilities|Casting|CastToShopInstance (Game|GetGameInstance)))
      (AddComponent|AddChildActorComponent false (Utilities|Array|Get(acopy) _diamondspawnpoints (Math|Random|RandomIntegerinRange 0 (Utilities|Array|LastIndex _diamondspawnpoints))))
      (Variables|/Game/SFTS/Blueprints/ShopInstance.ShopInstance_C|SetDiamondAlternater _asshop_instance_2 false))))

(fn LaserSpawnProbability
  (params (Percentage :type Integer))
  (return (== (Math|Random|RandomIntegerinRange 1 (Math|Integer|%(Integer) Percentage (Class|KismetSystemLibrary|MakeLiteralInteger 100))) 1)))