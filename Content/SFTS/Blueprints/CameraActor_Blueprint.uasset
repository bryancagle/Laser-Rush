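; Follow camera for the RunCharacter that becomes the player's view target on BeginPlay.
; Each Tick it locks X behind the player, eases Y and Z with fixed-step interpolation, and smooths pitch toward the player without sideways turning.
; Until ShopInstance flags Stage 1 complete, Y and Z are clamped to fixed bounds.
; Afterwards it follows unclamped and slightly faster, halting when StopCamera is set.
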(event Custom|MoveCamera)

(event EventBeginPlay
  ;[1 1 1] Camera follows player without being tied to the player's X and Y movement
  (bind _asrun_character (Utilities|Casting|CastToRunCharacter (Game|Player|GetPlayerPawn 0)))
  (bind _output_get (Variables|Default|SetMyPlayer _asrun_character))
  (bind _asplayer_controller (Utilities|Casting|CastToPlayerController (Pawn|GetController _output_get)))
  (Game|Player|SetViewTargetwithBlend _asplayer_controller self 0.0 "VTBlend_Cubic" 0.0 false)
  (Transformation|SetActorTransform (Math|Transform|MakeTransform (.location (Transformation|GetActorTransform (Variables|Default|GetMyPlayer))) (.rotation (Transformation|GetActorTransform (Variables|Default|GetMyPlayer))) "1,1,1")))

(event Collision|EventActorBeginOverlap
  (params (OtherActor :type Actor%20Object%20Reference)))

(event EventTick
  (params (DeltaSeconds :type Float%20%28single-precision%29))
  (bind _returnvalue (Transformation|GetActorRotation))
  (bind _returnvalue_2 (Transformation|GetActorLocation))
  (bind _returnvalue_3 (Transformation|GetActorLocation))
  (bind _returnvalue_4 (Transformation|GetActorLocation))
  (bind _myplayer (Variables|Default|GetMyPlayer))
  (bind _myplayer_2 (Variables|Default|GetMyPlayer))
  (bind _myplayer_3 (Variables|Default|GetMyPlayer))
  (bind _returnvalue_5 (Transformation|GetActorLocation _myplayer_2))
  (bind _returnvalue_6 (Transformation|GetActorLocation _myplayer))
  (bind _returnvalue_7 (Transformation|GetActorLocation _myplayer_3))
  (bind _returnvalue_8 (- _returnvalue_5 _returnvalue_2))
  (bind _returnvalue_9 (- _returnvalue_6 "500.000000,0.000000,-100.000000"))
  (bind _returnvalue_10 (- _returnvalue_7 "500.000000,0.000000,-100.000000"))
  (bind (_x _y _z) (Math|Vector|BreakVector _returnvalue_9))
  (bind (_x_2 _y_2 _z_2) (Math|Vector|BreakVector _returnvalue_10))
  (bind _returnvalue_11 (Math|Interpolation|VInterpTo (Math|Vector|MakeVector 0.0 (.y _returnvalue_3) (.z _returnvalue_3)) (Math|Vector|MakeVector 0.0 _y_2 _z_2) 0.1 0.5))
  (bind _returnvalue_12 (Math|Interpolation|VInterpTo (Math|Vector|MakeVector 0.0 (.y _returnvalue_4) (.z _returnvalue_4)) (Math|Vector|MakeVector 0.0 _y _z) 0.1 0.7))
  (bind _returnvalue_13 (Math|Float|Clamp(Float) (.z _returnvalue_11) 2.5e+02 7e+02))
  (bind _returnvalue_14 (Math|Float|Clamp(Float) (.y _returnvalue_11) -8.5e+02 8.5e+02))
  (bind _returnvalue_15 (Math|Vector|MakeVector _x_2 _returnvalue_14 _returnvalue_13))
  (bind _asshop_instance (Utilities|Casting|CastToShopInstance (Game|GetGameInstance)))
  (if (Variables|/Game/SFTS/Blueprints/ShopInstance.ShopInstance_C|GetStage1Complete _asshop_instance)
    (if (not (Variables|/Game/SFTS/Blueprints/ShopInstance.ShopInstance_C|GetStopCamera _asshop_instance))
      (Transformation|SetActorLocationAndRotation (Math|Vector|MakeVector _x (.y _returnvalue_12) (.z _returnvalue_12)) (Math|Interpolation|RInterpTo (Math|Rotator|MakeRotator 0.0 (.pitch _returnvalue) (.yaw _returnvalue)) (Math|Rotator|MakeRotator 0.0 (.pitch (Math|Conversions|RotationFromXVector (Math|Vector|MakeVector (.x _returnvalue_8) (Math|Float|Clamp(Float) (.y _returnvalue_8) 0.0 0.0) (Math|Float|Clamp(Float) (stale _result) -5e+01 0.0)))) (.yaw (Math|Conversions|RotationFromXVector (Math|Vector|MakeVector (.x _returnvalue_8) (Math|Float|Clamp(Float) (.y _returnvalue_8) 0.0 0.0) (Math|Float|Clamp(Float) (stale _result) -5e+01 0.0))))) 0.01 3.0)))
    (else
      (bind _result (Math|Float|NegateFloat (.z _returnvalue_8))
        (:%20%20
          (Transformation|SetActorLocationAndRotation (Math|Vector|MakeVector (.x _returnvalue_15) (.y _returnvalue_15) (.z _returnvalue_15)) (Math|Interpolation|RInterpTo (Math|Rotator|MakeRotator 0.0 (.pitch _returnvalue) (.yaw _returnvalue)) (Math|Rotator|MakeRotator 0.0 (.pitch (Math|Conversions|RotationFromXVector (Math|Vector|MakeVector (.x _returnvalue_8) (Math|Float|Clamp(Float) (.y _returnvalue_8) 0.0 0.0) (Math|Float|Clamp(Float) _result -5e+01 0.0)))) (.yaw (Math|Conversions|RotationFromXVector (Math|Vector|MakeVector (.x _returnvalue_8) (Math|Float|Clamp(Float) (.y _returnvalue_8) 0.0 0.0) (Math|Float|Clamp(Float) _result -5e+01 0.0))))) 0.01 3.0)))))))

(fn ConstructionScript)