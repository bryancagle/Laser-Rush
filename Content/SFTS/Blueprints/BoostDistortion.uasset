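; BoostDistortion is a short-lived effect actor that spawns as an expanding flat distortion at the player's position, apparently for a boost.
; BeginPlay snaps it to the player pawn once, zeroes its scale and destroys it after a half-second delay.
; Tick adds a fixed step to X and Y scale, leaving Z at zero, so growth depends on frame rate.
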(event EventBeginPlay
  (bind _returnvalue (Game|Player|GetPlayerPawn 0))
  (bind _returnvalue_2 (Transformation|GetActorLocation _returnvalue))
  ;[1 1 1] When it is created, it follows the player, expands, then removes itself
  (Transformation|SetActorLocation (Math|Vector|MakeVector (.x _returnvalue_2) (.y _returnvalue_2) (+ (.z _returnvalue_2) 0.0)) false false)
  (Transformation|SetActorScale3D "0.000000,0.000000,0.000000")
  (Utilities|FlowControl|Delay 0.5)
  (Actor|DestroyActor))

(event Collision|EventActorBeginOverlap
  (params (OtherActor :type Actor%20Object%20Reference))
  ;[1 1 1] When it is created, it follows the player, expands, then removes itself
)

(event EventTick
  (params (DeltaSeconds :type Float%20%28single-precision%29))
  ;[1 1 1] When it is created, it follows the player, expands, then removes itself
  (Transformation|SetActorScale3D (+ (Transformation|GetActorScale3D) "1.000000,1.000000,0.000000")))

(fn ConstructionScript)